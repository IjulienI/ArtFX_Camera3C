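; BP_2D is a Fez-style player actor that turns in 90-degree steps.
; On BeginPlay it spawns a BP_BaseCamera, stores it as PlayerCamera and makes it player 0's view target.
; TurnCamera plays the TurnCam timeline to lerp the actor's own yaw by -90 degrees from its starting value.
; CanMove is false during the turn and is restored when the timeline finishes.
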(event `self.ReceiveBeginPlay`
  (bind _returnvalue (`|SpawnActorFromClass` "/Game/_Base/Fez/BP_BaseCamera.BP_BaseCamera_C" (`KismetMathLibrary.MakeTransform` (0.0 0.0 0.0)) "Undefined" "MultiplyWithRoot" null self null))
  (bind _output_get (set `self.PlayerCamera` _returnvalue))
  (`PlayerController.SetViewTargetWithBlend` (`GameplayStatics.GetPlayerController` 0) _output_get 0.0 "VTBlend_Linear" 0.0 false))

(event `TurnCamera`
  (bind (_returnvalue_roll _returnvalue_pitch _returnvalue_yaw) (`KismetMathLibrary.BreakRotator` (`self.K2_GetActorRotation`)))
  (bind _initialplayerrot (`self.InitialPlayerRot`))
  (set `self.bCanMove` false)
  (set `self.InitialPlayerRot` _returnvalue_yaw)
  (bind (_direction _camerarot) (`Timeline|TurnCam` :!via `PlayFromStart`)
    (:`Update`
      (`self.K2_SetActorRotation` (`KismetMathLibrary.MakeRotator` 0.0 0.0 (`KismetMathLibrary.Lerp` _initialplayerrot (+ _initialplayerrot -90.0) _camerarot))))
    (:`Finished`
      (set `self.bCanMove` true))))

(fn `UserConstructionScript`)