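; Fez-style orthographic follow camera that turns around the player in animated yaw steps, configured at BeginPlay from DT_FezCamera.
; Tick eases it toward an offset target that always tracks player height but only fully recenters when the camera-to-player distance exceeds a dead zone.
; AddRotation freezes the player during a timeline turn, carrying over unfinished rotation from interrupted turns.
; EndRotation realigns the player and restores gravity, control and the saved velocity rotated by the turn.
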(event `self.ReceiveBeginPlay`
  (`self.ApplyData`)
  (`self.SetTargetAsPlayerPos`))

(event `self.ReceiveTick`
  (params (DeltaSeconds :type "Float (single-precision)"))
  (`self.K2_SetActorLocation` (`KismetMathLibrary.VInterpTo` (`self.K2_GetActorLocation`) (+ (`self.TargetPoint`) (`self.Offset`)) (`GameplayStatics.GetWorldDeltaSeconds`) (`self.CameraLagSpeed`)))
  (set `self.TargetPoint` (`KismetMathLibrary.MakeVector` (.x (`self.TargetPoint`)) (.y (`self.TargetPoint`)) (.z (`self.K2_GetActorLocation` (`self.TargetRef`)))))
  (if (not (<= (`KismetMathLibrary.Vector_Distance` (`self.K2_GetActorLocation`) (`self.K2_GetActorLocation` (`self.TargetRef`))) (`self.DeadZone`)))
    (`self.SetTargetAsPlayerPos`)))

(event `AddRotation`
  (params (Rotation :type "Float (double-precision)"))
  (bind (_returnvalue_roll _returnvalue_pitch) (`KismetMathLibrary.BreakRotator` (`self.K2_GetActorRotation`)))
  (bind _initialrotation (`self.InitialRotation`))
  (bind _targetref (`self.TargetRef`))
  (bind _charactermovement (`Character.CharacterMovement` _targetref))
  (set `/Game/_Base/Fez/BP_2D.bCanMove` false _targetref)
  (set `self.InitialVelocity` (`MovementComponent.Velocity` _charactermovement))
  (set `CharacterMovementComponent.GravityScale` 0.0 _charactermovement)
  (`MovementComponent.StopMovementImmediately` _charactermovement)
  (set `self.PendingRotation` Rotation)
  (set `self.InitialRotation` (.yaw (`self.K2_GetActorRotation`)))
  (set `self.PendingRotation` (+ (`self.PendingRotation`) (`self.TempPendingRotation`)))
  (`TimelineComponent.SetPlayRate` (`self.CameraRotation`) (/ 1.0 (`self.TurnSpeed`)))
  (bind (_direction _rotation) (`Timeline|CameraRotation` :!via `PlayFromStart`)
    (:`Update`
      (set `self.TempPendingRotation` (`KismetMathLibrary.Lerp` (`self.PendingRotation`) 0.0 _rotation))
      (`self.K2_SetActorRotation` (`KismetMathLibrary.MakeRotator` _returnvalue_roll _returnvalue_pitch (`KismetMathLibrary.Lerp` _initialrotation (+ _initialrotation (`self.PendingRotation`)) _rotation))))
    (:`Finished`
      (`self.EndRotation`))))

(event `EndRotation`
  (bind (_returnvalue_roll _returnvalue_pitch _returnvalue_yaw) (`KismetMathLibrary.BreakRotator` (`self.K2_GetActorRotation`)))
  (bind (_returnvalue_roll_2 _returnvalue_pitch_2 _returnvalue_yaw_2) (`KismetMathLibrary.BreakRotator` (`self.K2_GetActorRotation`)))
  (bind _targetref (`self.TargetRef`))
  (bind _charactermovement (`Character.CharacterMovement` (`self.TargetRef`)))
  (`self.K2_SetActorRotation` _targetref (`KismetMathLibrary.MakeRotator` 0.0 0.0 _returnvalue_yaw_2) false)
  (set `MovementComponent.Velocity` (`KismetMathLibrary.GreaterGreater_VectorRotator` (`self.InitialVelocity`) (`KismetMathLibrary.MakeRotator` 0.0 0.0 (- _returnvalue_yaw (`self.InitialRotation`)))) _charactermovement)
  (set `CharacterMovementComponent.GravityScale` 1.0 _charactermovement)
  (set `/Game/_Base/Fez/BP_2D.bCanMove` true _targetref))

(fn `ApplyData`
  (bind _springarm (`self.SpringArm`))
  (bind _outrownames (`DataTableFunctionLibrary.GetDataTableRowNames` "/Game/_Game/Fez/DT_FezCamera.DT_FezCamera"))
  (for _array_element _outrownames
    (bind _returnvalue (`|GetDataTableRow` "/Game/_Game/Fez/DT_FezCamera.DT_FezCamera" _array_element)
      (:`then`
        (bind (_orthowidth _offset _rotationspeed _lag _lagspeed _deadzone) (break `/Game/_Base/Fez/Struct_FezCamera` _returnvalue))
        (`CameraComponent.SetOrthoWidth` (`self.Camera`) _orthowidth)
        (set `self.Offset` _offset)
        (set `self.TurnSpeed` _rotationspeed)
        (set `SpringArmComponent.bEnableCameraLag` _lag _springarm)
        (set `SpringArmComponent.CameraLagSpeed` _lagspeed _springarm)
        (set `self.DeadZone` _deadzone)))))

(fn `SetTargetAsPlayerPos`
  (set `self.TargetPoint` (`self.K2_GetActorLocation` (`self.TargetRef`))))

(fn `UserConstructionScript`)